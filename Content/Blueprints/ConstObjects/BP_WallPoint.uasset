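; BP_WallPoint is a wall object with a cube mesh whose texture, color and grid mask can be changed at runtime.
; On BeginPlay it creates a dynamic material instance on the cube and turns the mask fully on.
; Events then set that instance's texture, MaskOpacity and color parameters.
; GetWallFace converts a hit location into cube local space and uses the sign of X to return which face was hit.
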(event `self.ReceiveBeginPlay`
  (`parent.ReceiveBeginPlay`)
  (bind _returnvalue (`PrimitiveComponent.CreateDynamicMaterialInstance` (`self.Cube`) 0 "/Game/Materials/M_DynamicMaterial.M_DynamicMaterial" "None"))
  (bind _output_get (set `self.DynamicMaterial` _returnvalue))
  (`MaterialInstanceDynamic.SetScalarParameterValue` _output_get "MaskOpacity" 1.0))

(event `ChangeTexture`
  (params (Texture :type "Texture2D Object Reference"))
  (`MaterialInstanceDynamic.SetTextureParameterValue` (`self.DynamicMaterial`) "TextureParameter" Texture))

(event `SwitchGrid`
  (params (Mode :type "Float (double-precision)"))
  (`MaterialInstanceDynamic.SetScalarParameterValue` (`self.DynamicMaterial`) "MaskOpacity" Mode))

(event `ColorApply`
  (params (Color :type "LinearColor Structure"))
  (`MaterialInstanceDynamic.SetVectorParameterValue` (`self.DynamicMaterial`) "ColorParam" Color))

(fn `GetWallFace`
  (params (HitLocation :type "Vector Structure"))
  (returns (Face :type Integer))
  (locals (FaceID :type Integer :default 0))
  (bind _returnvalue_x (`KismetMathLibrary.BreakVector` (`KismetMathLibrary.InverseTransformLocation` (`SceneComponent.K2_GetComponentToWorld` (`self.Cube`)) HitLocation)))
  (`|ExecutionSequence`
    (:`then_0`
      (if (> _returnvalue_x 0.0)
        (set `local.FaceID` 1)
        (else
          (set `local.FaceID` 0))))
    (:`then_1`
      (return (`local.FaceID`)))))

(fn `UserConstructionScript`
  (`parent.UserConstructionScript`))