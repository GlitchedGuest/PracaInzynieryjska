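; Handheld tablet actor for a room-building tool, with a laser pointer, a switchable widget screen and a gizmo for placing objects.
; A pointer line trace finds wall points for retexturing or for spawning construction objects, validated by wall tags.
; Each tick updates the beam and gizmo overlap material, and moves the tracked door, window, ceiling object or new wall with grid snapping.
; Wall dimensions and rotation come live from the details widget.
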(event `TurnLaser`
  (params (Mode :type Boolean))
  (`SceneComponent.SetVisibility` (`self.Laser`) Mode false))

(event `self.ReceiveTick`
  (params (DeltaSeconds :type "Float (single-precision)"))
  (bind _cube1 (`self.Cube1`))
  (bind _pointer (`self.Pointer`))
  (bind _returnvalue (`SceneComponent.K2_GetComponentLocation` _pointer))
  (`|ExecutionSequence`
    (:`then_0`
      (bind _output_get (set `self.Blocked` (`KismetArrayLibrary.Array_IsNotEmpty` (`PrimitiveComponent.GetOverlappingActors` (`self.Cube1`) "/Script/Engine.Actor"))))
      (if _output_get
        (`PrimitiveComponent.SetMaterial` _cube1 0 "/Game/Materials/M_CollBad.M_CollBad")
        (else
          (`PrimitiveComponent.SetMaterial` _cube1 0 "/Game/Materials/M_CollGood.M_CollGood"))))
    (:`then_1`
      (`self.UpdateConstObjects`))
    (:`then_2`
      (bind _outactors (`GameplayStatics.GetAllActorsOfClass` "/Game/Blueprints/BP_ObjectParent.BP_ObjectParent_C"))
      (bind _outhit (`KismetSystemLibrary.LineTraceSingle` _returnvalue (+ _returnvalue (* (`SceneComponent.GetForwardVector` _pointer) (`self.TabletRange`))) "TraceTypeQuery1" false _outactors))
      (`FXSystemComponent.SetVectorParameter` (`self.Laser`) "Beam End" (`KismetMathLibrary.MakeVector` (`KismetMathLibrary.Vector_Distance` (`SceneComponent.K2_GetComponentLocation` (`self.Pointer`)) (`.ImpactPoint` (`GameplayStatics.BreakHitResult` _outhit))))))))

(event `self.ReceiveBeginPlay`
  (`FXSystemComponent.SetColorParameter` (`self.Laser`) "Color" (`self.LaserColor`)))

(event `SwitchWidget`
  (params (Index :type Integer))
  (bind _aswb_tablet_switcher (cast `/Game/Widgets/WB_TabletSwitcher` (`WidgetComponent.GetWidget` (`self.Widget`))))
  (`/Game/Widgets/WB_TabletSwitcher.SwitchWidget` _aswb_tablet_switcher Index))

(event `HideGizmo`
  (`SceneComponent.SetVisibility` (`self.Cube1`) false false))

(event `SetGizmo`
  (params (Mesh :type "StaticMesh Object Reference") (Scale :type "Vector Structure"))
  (bind _cube1 (`self.Cube1`))
  (`StaticMeshComponent.SetStaticMesh` _cube1 Mesh)
  (`SceneComponent.SetVisibility` _cube1 true false)
  (`SceneComponent.SetWorldScale3D` _cube1 Scale))

(event `ScaleGizmo`
  (params (ScaleDir :type "Float (double-precision)"))
  (bind _returnvalue (* ScaleDir 0.1))
  (bind _cube1 (`self.Cube1`))
  (bind (_returnvalue_x _returnvalue_y _returnvalue_z) (`KismetMathLibrary.BreakVector` (`SceneComponent.K2_GetComponentScale` _cube1)))
  (bind _returnvalue_2 (+ _returnvalue_x _returnvalue))
  (if (>= _returnvalue_2 0.1)
    (`SceneComponent.SetWorldScale3D` _cube1 (`KismetMathLibrary.MakeVector` _returnvalue_2 (+ _returnvalue_y _returnvalue) (+ _returnvalue_z _returnvalue)))))

(event `Spawn`
  (bind _cube1 (`self.Cube1`))
  (bind _returnvalue (`|SpawnActorFromClass` "/Game/Blueprints/BP_ObjectParent.BP_ObjectParent_C" (`KismetMathLibrary.MakeTransform` (`SceneComponent.K2_GetComponentLocation` _cube1) (`SceneComponent.K2_GetComponentRotation` _cube1) (`SceneComponent.K2_GetComponentScale` (`self.Cube1`))) "Undefined" "MultiplyWithRoot" null null))
  (`StaticMeshComponent.SetStaticMesh` (`/Game/Blueprints/BP_ObjectParent.StaticMesh` _returnvalue) (`self.Mesh`))
  (`SceneComponent.SetVisibility` _cube1 false false))

(event `CancelConstObject`
  (if (== (`self.CObjectType`) 5)
    (set `self.CObjectType` -1)
    (`self.K2_DestroyActor` (`self.TrackObject`) :!label _label)
    (elif (`self.TrackObjectCheck`)
      (set `self.TrackObjectCheck` false)
      (goto _label))))

(event `ChangeMaterial`
  (params (Texture :type "Texture2D Object Reference"))
  (bind (_location _wall) (`self.TraceLine`))
  (`/Game/Blueprints/ConstObjects/BP_WallPoint.ChangeTexture` _wall Texture)
  (set `self.TrackedWall` _wall)
  (`self.SwitchWidget` 3))

(fn `CreateWall`
  (params (Mode :type Boolean))
  (if Mode
    (set `self.CObjectType` 5)
    (else
      (set `self.CObjectType` -1)))
  (set `self.TrackObjectCheck` Mode))

(fn `FollowObjectToWall`)

(fn `SpawnConstObject`
  (params (CObjectType :type Integer) (ObjectClass :type "Actor Class Reference"))
  (returns (Success :type Boolean))
  (bind _output_get (set `self.CObjectType` CObjectType))
  (if (`self.TrackObjectCheck`)
    (set `self.TrackObjectCheck` false)
    (else
      (switch `int` _output_get
        (:`1`
          (bind (_location _wall) (`self.TraceLine` :!label _label))
          (bind _face (`/Game/Blueprints/ConstObjects/BP_WallPoint.GetWallFace` _wall (`KismetMathLibrary.MakeVector` (.x _location) (.y _location) (.z _location))))
          (bind _tags (`Actor.Tags` _wall))
          (if (or (`KismetArrayLibrary.Array_Contains` _tags "North") (`KismetArrayLibrary.Array_Contains` _tags "East") (`KismetArrayLibrary.Array_Contains` _tags "West") (`KismetArrayLibrary.Array_Contains` _tags "South"))
            (bind _returnvalue (`self.K2_GetActorRotation` _wall))
            (bind _returnvalue_2 (`|SpawnActorFromClass` ObjectClass (`KismetMathLibrary.MakeTransform` (`KismetMathLibrary.MakeVector` (.x _location) (.y _location)) (`KismetMathLibrary.ComposeRotators` _returnvalue (`KismetMathLibrary.MakeRotator` 0.0 0.0 (`KismetMathLibrary.Conv_IntToDouble` (* _face 180))))) "AlwaysSpawn" "MultiplyWithRoot" null null))
            (bind _asbp_const_object (cast `/Game/Blueprints/ConstObjects/BP_ConstObject` _returnvalue_2))
            (set `self.TrackObjectCheck` true)
            (set `self.TrackObject` _asbp_const_object)
            (set `self.TrackedWall` _wall)
            (set `self.ConstZRotation` (.yaw _returnvalue))
            (return true)
            (else
              _)))
        (:`2`
          (goto _label))
        (:`3`
          (bind (_location_2 _wall_2) (`self.TraceLine`))
          (if (`KismetArrayLibrary.Array_Contains` (`Actor.Tags` _wall_2) "ZOffset")
            (bind _returnvalue_3 (`|SpawnActorFromClass` ObjectClass (`KismetMathLibrary.MakeTransform` (`KismetMathLibrary.MakeVector` (.x _location_2) (.y _location_2) (.z _location_2))) "AlwaysSpawn" "MultiplyWithRoot" null null))
            (bind _asbp_const_object_2 (cast `/Game/Blueprints/ConstObjects/BP_ConstObject` _returnvalue_3))
            (set `self.TrackObjectCheck` true)
            (set `self.TrackObject` _asbp_const_object_2)
            (set `self.TrackedWall` _wall_2)
            (return true)
            (else
              _))))
      (return false))))

(fn `SpawnWallObject`
  (returns (Success :type Boolean))
  (set `self.CObjectType` 4)
  (if (`self.TrackObjectCheck`)
    (set `self.TrackObjectCheck` false)
    (else
      (bind (_location _wall) (`self.TraceLine`))
      (bind _tags (`Actor.Tags` _wall))
      (if (and (`KismetArrayLibrary.Array_Contains` _tags "Floor") (== (`KismetArrayLibrary.Array_Length` _tags) 1))
        (bind _outactors (`GameplayStatics.GetAllActorsOfClassWithTag` "/Game/Blueprints/ConstObjects/BP_WallPoint.BP_WallPoint_C" "North"))
        (bind _returnvalue (`KismetMathLibrary.Round` (.x _location)))
        (bind _returnvalue_2 (`KismetMathLibrary.Round` (.y _location)))
        (bind (_returnvalue_x _returnvalue_y _returnvalue_z) (`KismetMathLibrary.BreakVector` (`self.GetActorScale3D` (`|GetArrayItem` _outactors))))
        (bind _returnvalue_3 (`|SpawnActorFromClass` "/Game/Blueprints/ConstObjects/BP_WallPoint.BP_WallPoint_C" (`KismetMathLibrary.MakeTransform` (`KismetMathLibrary.MakeVector` (`KismetMathLibrary.Conv_IntToDouble` (- _returnvalue (mod _returnvalue 10))) (`KismetMathLibrary.Conv_IntToDouble` (- _returnvalue_2 (mod _returnvalue_2 10)))) (struct) (`KismetMathLibrary.MakeVector` 0.2 0.2 (- _returnvalue_z 0.3))) "AlwaysSpawn" "MultiplyWithRoot" null null))
        (set `self.TrackObjectCheck` true)
        (set `self.TrackObject` _returnvalue_3)
        (return true)
        (else
          (return false))))))

(fn `TraceLine`
  (returns (Location :type "Vector Structure") (Wall :type "/Game/Blueprints/ConstObjects/BP_WallPoint Object Reference"))
  (bind _ignorable (`self.Ignorable`))
  (bind _pointer (`self.Pointer`))
  (bind _returnvalue (`SceneComponent.K2_GetComponentLocation` _pointer))
  (`KismetArrayLibrary.Array_Clear` (`self.Ignorable`))
  (bind _outactors (`GameplayStatics.GetAllActorsOfClass` "/Game/Blueprints/ConstObjects/BP_ConstDecoration.BP_ConstDecoration_C"))
  (for _array_element _outactors
    (`KismetArrayLibrary.Array_Add` _ignorable _array_element))
  (bind _outactors_2 (`GameplayStatics.GetAllActorsOfClass` "/Game/Blueprints/BP_ObjectParent.BP_ObjectParent_C"))
  (for _array_element_2 _outactors_2
    (`KismetArrayLibrary.Array_Add` _ignorable _array_element_2))
  (bind _outhit (`KismetSystemLibrary.LineTraceSingle` _returnvalue (+ _returnvalue (* (`SceneComponent.GetForwardVector` _pointer) (`self.TabletRange`))) "TraceTypeQuery1" false (`self.Ignorable`)))
  (bind (_bblockinghit _binitialoverlap _time _distance _location _impactpoint _normal _impactnormal _physmat _hitactor) (`GameplayStatics.BreakHitResult` _outhit))
  (bind _asbp_wall_point (cast `/Game/Blueprints/ConstObjects/BP_WallPoint` _hitactor))
  (return _impactpoint _asbp_wall_point))

(fn `UpdateCeilingObjectType`
  (params (Location :type "Vector Structure") (`Tracked Object` :type "/Game/Blueprints/ConstObjects/BP_ConstObject Object Reference") (`Hit Object` :type "/Game/Blueprints/ConstObjects/BP_WallPoint Object Reference"))
  (locals (NewLocation :type "Vector Structure"))
  (bind _x (.x Location))
  (bind _y (.y Location))
  (bind (_newlocation_x _newlocation_y _newlocation_z) (`KismetMathLibrary.BreakVector` (`local.NewLocation`)))
  (bind _defaultsceneroot (`/Game/Blueprints/ConstObjects/BP_ConstObject.DefaultSceneRoot` `Tracked Object`))
  (bind (_newlocation_x_2 _newlocation_y_2 _newlocation_z_2) (`KismetMathLibrary.BreakVector` (`local.NewLocation`)))
  (bind _returnvalue (`KismetMathLibrary.Round` _y))
  (bind _returnvalue_2 (`KismetMathLibrary.Round` _x))
  (bind (_returnvalue_x _returnvalue_y _returnvalue_z) (`KismetMathLibrary.BreakVector` (`SceneComponent.K2_GetComponentLocation` _defaultsceneroot)))
  (if (== (`self.TrackedWall`) `Hit Object`)
    (set `local.NewLocation` (`KismetMathLibrary.MakeVector` _returnvalue_x _returnvalue_y _returnvalue_z))
    (`|ExecutionSequence`
      (:`then_0`
        (if (>= (`KismetMathLibrary.Abs` (- _returnvalue_x _x)) (`KismetMathLibrary.Conv_IntToDouble` (`self.GridMagnetStrength`)))
          (set `local.NewLocation` (`KismetMathLibrary.MakeVector` (`KismetMathLibrary.Conv_IntToDouble` (- _returnvalue_2 (mod _returnvalue_2 (`self.GridMagnetStrength`)))) _newlocation_y_2 _newlocation_z_2))))
      (:`then_1`
        (if (>= (`KismetMathLibrary.Abs` (- _returnvalue_y _y)) (`KismetMathLibrary.Conv_IntToDouble` (`self.GridMagnetStrength`)))
          (set `local.NewLocation` (`KismetMathLibrary.MakeVector` _newlocation_x (`KismetMathLibrary.Conv_IntToDouble` (- _returnvalue (mod _returnvalue (`self.GridMagnetStrength`)))) _newlocation_z))))
      (:`then_2`
        (`SceneComponent.K2_SetWorldLocation` _defaultsceneroot (`local.NewLocation`) false false)))))

(fn `UpdateConstObjects`
  (bind _trackobject (`self.TrackObject`))
  (bind (_returnvalue_roll _returnvalue_pitch) (`KismetMathLibrary.BreakRotator` (`SceneComponent.K2_GetComponentRotation` (`/Game/Blueprints/ConstObjects/BP_ConstObject.DefaultSceneRoot` _trackobject))))
  (if (`self.TrackObjectCheck`)
    (bind (_location _wall) (`self.TraceLine`))
    (switch `int` (`self.CObjectType`)
      (:`1`
        (`self.UpdateDoorObjectType` _wall _location _trackobject)
        (bind _face (`/Game/Blueprints/ConstObjects/BP_WallPoint.GetWallFace` (`self.TrackedWall`) _location :!label _label))
        (`SceneComponent.K2_SetWorldRotation` (`Actor.RootComponent` _trackobject) (`KismetMathLibrary.MakeRotator` _returnvalue_roll _returnvalue_pitch (+ (`self.ConstZRotation`) (* _face 180.0))) false false))
      (:`2`
        (`self.UpdateWindowObjectType` _location _wall _trackobject)
        (goto _label))
      (:`3`
        (`self.UpdateCeilingObjectType` _location _trackobject _wall))
      (:`4`
        (`self.UpdateWallObjectType` _location _trackobject))
      (:`5`
        (`self.UpdateDimensionWallObjectType`)))))

(fn `UpdateDimensionWallObjectType`
  (bind _trackobject (`self.TrackObject`))
  (bind (_returnvalue_x _returnvalue_y _returnvalue_z) (`KismetMathLibrary.BreakVector` (`self.GetActorScale3D` _trackobject)))
  (bind (_returnvalue_roll _returnvalue_pitch) (`KismetMathLibrary.BreakRotator` (`self.K2_GetActorRotation` _trackobject)))
  (bind _aswb_tablet_switcher (cast `/Game/Widgets/WB_TabletSwitcher` (`WidgetComponent.GetWidget` (`self.Widget`))))
  (bind _aswb_const_wall_details (cast `/Game/Widgets/WB_ConstWallDetails` (`WidgetSwitcher.GetActiveWidget` (`/Game/Widgets/WB_TabletSwitcher.WidgetSwitcher` _aswb_tablet_switcher))))
  (`self.SetActorScale3D` _trackobject (`KismetMathLibrary.MakeVector` (`/Game/Widgets/WB_ConstWallDetails.Width` _aswb_const_wall_details) (`/Game/Widgets/WB_ConstWallDetails.Length` _aswb_const_wall_details) _returnvalue_z))
  (`self.K2_SetActorRotation` _trackobject (`KismetMathLibrary.MakeRotator` _returnvalue_roll _returnvalue_pitch (`/Game/Widgets/WB_ConstWallDetails.Rotation` _aswb_const_wall_details)) false))

(fn `UpdateDoorObjectType`
  (params (HitObject :type "Object Object Reference") (Location :type "Vector Structure") (TrackedObject :type "/Game/Blueprints/ConstObjects/BP_ConstObject Object Reference"))
  (locals (NewLocation :type "Vector Structure"))
  (bind _returnvalue (`KismetMathLibrary.Round` Location_Y))
  (bind _returnvalue_2 (`KismetMathLibrary.Round` Location_X))
  (bind _newlocation_x (`KismetMathLibrary.BreakVector` (`local.NewLocation`)))
  (bind _defaultsceneroot (`/Game/Blueprints/ConstObjects/BP_ConstObject.DefaultSceneRoot` TrackedObject))
  (bind (_newlocation_x_2 _newlocation_y) (`KismetMathLibrary.BreakVector` (`local.NewLocation`)))
  (bind (_returnvalue_x _returnvalue_y) (`KismetMathLibrary.BreakVector` (`SceneComponent.K2_GetComponentLocation` _defaultsceneroot)))
  (if (== (`self.TrackedWall`) HitObject)
    (set `local.NewLocation` (`KismetMathLibrary.MakeVector` _returnvalue_x _returnvalue_y))
    (`|ExecutionSequence`
      (:`then_0`
        (if (>= (`KismetMathLibrary.Abs` (- _returnvalue_x Location_X)) (`KismetMathLibrary.Conv_IntToDouble` (`self.GridMagnetStrength`)))
          (set `local.NewLocation` (`KismetMathLibrary.MakeVector` (`KismetMathLibrary.Conv_IntToDouble` (- _returnvalue_2 (mod _returnvalue_2 (`self.GridMagnetStrength`)))) _newlocation_y))))
      (:`then_1`
        (if (>= (`KismetMathLibrary.Abs` (- _returnvalue_y Location_Y)) (`KismetMathLibrary.Conv_IntToDouble` (`self.GridMagnetStrength`)))
          (set `local.NewLocation` (`KismetMathLibrary.MakeVector` _newlocation_x (`KismetMathLibrary.Conv_IntToDouble` (- _returnvalue (mod _returnvalue (`self.GridMagnetStrength`))))))))
      (:`then_2`
        (`SceneComponent.K2_SetWorldLocation` _defaultsceneroot (`local.NewLocation`) false false)))))

(fn `UpdateWallObjectType`
  (params (Location :type "Vector Structure") (`Tracked Object` :type "/Game/Blueprints/ConstObjects/BP_ConstObject Object Reference"))
  (locals (NewLocation :type "Vector Structure"))
  (bind _x (.x Location))
  (bind _y (.y Location))
  (bind (_newlocation_x _newlocation_y _newlocation_z) (`KismetMathLibrary.BreakVector` (`local.NewLocation`)))
  (bind _defaultsceneroot (`/Game/Blueprints/ConstObjects/BP_ConstObject.DefaultSceneRoot` `Tracked Object`))
  (bind (_newlocation_x_2 _newlocation_y_2 _newlocation_z_2) (`KismetMathLibrary.BreakVector` (`local.NewLocation`)))
  (bind _returnvalue (`KismetMathLibrary.Round` _x))
  (bind _returnvalue_2 (`KismetMathLibrary.Round` _y))
  (bind (_returnvalue_x _returnvalue_y _returnvalue_z) (`KismetMathLibrary.BreakVector` (`SceneComponent.K2_GetComponentLocation` _defaultsceneroot)))
  (set `local.NewLocation` (`KismetMathLibrary.MakeVector` _returnvalue_x _returnvalue_y _returnvalue_z))
  (`|ExecutionSequence`
    (:`then_0`
      (if (>= (`KismetMathLibrary.Abs` (- _returnvalue_x _x)) (`KismetMathLibrary.Conv_IntToDouble` (`self.GridMagnetStrength`)))
        (set `local.NewLocation` (`KismetMathLibrary.MakeVector` (`KismetMathLibrary.Conv_IntToDouble` (- _returnvalue (mod _returnvalue (`self.GridMagnetStrength`)))) _newlocation_y_2 _newlocation_z_2))))
    (:`then_1`
      (if (>= (`KismetMathLibrary.Abs` (- _returnvalue_y _y)) (`KismetMathLibrary.Conv_IntToDouble` (`self.GridMagnetStrength`)))
        (set `local.NewLocation` (`KismetMathLibrary.MakeVector` _newlocation_x (`KismetMathLibrary.Conv_IntToDouble` (- _returnvalue_2 (mod _returnvalue_2 (`self.GridMagnetStrength`)))) _newlocation_z))))
    (:`then_2`
      (`SceneComponent.K2_SetWorldLocation` _defaultsceneroot (`local.NewLocation`) false false))))

(fn `UpdateWindowObjectType`
  (params (Location :type "Vector Structure") (HitObject :type "Object Object Reference") (TrackedObject :type "/Game/Blueprints/ConstObjects/BP_ConstObject Object Reference"))
  (locals (NewLocation :type "Vector Structure"))
  (bind _returnvalue (`KismetMathLibrary.Round` Location_Y))
  (bind _returnvalue_2 (`KismetMathLibrary.Round` Location_Z))
  (bind _returnvalue_3 (`KismetMathLibrary.Round` Location_X))
  (bind (_newlocation_x _newlocation_y _newlocation_z) (`KismetMathLibrary.BreakVector` (`local.NewLocation`)))
  (bind (_newlocation_x_2 _newlocation_y_2) (`KismetMathLibrary.BreakVector` (`local.NewLocation`)))
  (bind _defaultsceneroot (`/Game/Blueprints/ConstObjects/BP_ConstObject.DefaultSceneRoot` TrackedObject))
  (bind (_newlocation_x_3 _newlocation_y_3 _newlocation_z_2) (`KismetMathLibrary.BreakVector` (`local.NewLocation`)))
  (bind (_returnvalue_x _returnvalue_y _returnvalue_z) (`KismetMathLibrary.BreakVector` (`SceneComponent.K2_GetComponentLocation` _defaultsceneroot)))
  (if (== (`self.TrackedWall`) HitObject)
    (set `local.NewLocation` (`KismetMathLibrary.MakeVector` _returnvalue_x _returnvalue_y _returnvalue_z))
    (`|ExecutionSequence`
      (:`then_0`
        (if (>= (`KismetMathLibrary.Abs` (- _returnvalue_x Location_X)) (`KismetMathLibrary.Conv_IntToDouble` (`self.GridMagnetStrength`)))
          (set `local.NewLocation` (`KismetMathLibrary.MakeVector` (`KismetMathLibrary.Conv_IntToDouble` (- _returnvalue_3 (mod _returnvalue_3 (`self.GridMagnetStrength`)))) _newlocation_y_3 _newlocation_z_2))))
      (:`then_1`
        (if (>= (`KismetMathLibrary.Abs` (- _returnvalue_y Location_Y)) (`KismetMathLibrary.Conv_IntToDouble` (`self.GridMagnetStrength`)))
          (set `local.NewLocation` (`KismetMathLibrary.MakeVector` _newlocation_x (`KismetMathLibrary.Conv_IntToDouble` (- _returnvalue (mod _returnvalue (`self.GridMagnetStrength`)))) _newlocation_z))))
      (:`then_2`
        (if (>= (`KismetMathLibrary.Abs` (- _returnvalue_z Location_Z)) (`KismetMathLibrary.Conv_IntToDouble` (`self.GridMagnetStrength`)))
          (set `local.NewLocation` (`KismetMathLibrary.MakeVector` _newlocation_x_2 _newlocation_y_2 (`KismetMathLibrary.Conv_IntToDouble` (- _returnvalue_2 (mod _returnvalue_2 (`self.GridMagnetStrength`))))))))
      (:`then_3`
        (`SceneComponent.K2_SetWorldLocation` _defaultsceneroot (`local.NewLocation`) false false)))))

(fn `UserConstructionScript`)